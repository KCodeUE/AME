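; Butterfly pickup actor that plays a looping flight animation and vanishes when its sphere is touched.
; BeginPlay starts the animation on the skeletal mesh.
; Any sphere overlap destroys the actor, spawns a smoke emitter and calls play sound at its location, with no sound asset set.
; ButterfliesCaught increments ButterflyScore and calls itself without an exit condition, and nothing in this graph triggers it.
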(event `ButterfliesCaught`
  (set `self.Butterfly Score` (+ (`self.Butterfly Score`) 1))
  (`self.ButterfliesCaught`))

(event `self.Sphere.OnComponentBeginOverlap`
  (params (OverlappedComponent :type "PrimitiveComponent Object Reference") (OtherActor :type "Actor Object Reference") (OtherComp :type "PrimitiveComponent Object Reference") (OtherBodyIndex :type Integer) (bFromSweep :type Boolean) (SweepResult :type "HitResult Structure (by ref)"))
  (bind _returnvalue (`self.K2_GetActorLocation`))
  (`self.K2_DestroyActor`)
  (`GameplayStatics.SpawnEmitterAtLocation` "/Game/StarterContent/Particles/P_Smoke.P_Smoke" _returnvalue)
  (`GameplayStatics.PlaySoundAtLocation` null _returnvalue))

(event `self.ReceiveBeginPlay`
  (`SkeletalMeshComponent.PlayAnimation` (`self.SkeletalMesh`) "/Game/Butterfly/Butterfly/Butterfly_Anim.Butterfly_Anim" true))

(fn `UserConstructionScript`)